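; AI controller for a team deathmatch agent that runs BT_TDMAgent and turns perception events into blackboard values and hero states.
; Sight of an affiliation-checked hero, or damage from one, focuses the nearest target, with sighting also setting state by weapon optimal range.
; Damage updates a low-health flag, while sensed health and weapon pads record pickup positions.
; Death clears the blackboard keys, and the hearing handler is left unconnected.
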(event `self.ReceivePossess`
  (params (PossessedPawn :type "Pawn Object Reference"))
  (`parent.ReceivePossess` PossessedPawn)
  (`self.RunBehaviorTree` "/Game/1_AIAG_Shooter/AI/AITeams/TimeVerde/BT_TDMAgent.BT_TDMAgent")
  (`/Game/1_AIAG_Shooter/Characters/BP_Hero.Character Set State` (`self.GetControlledHero`) "NewEnumerator1"))

(event `self.AIPerception.OnTargetPerceptionUpdated`
  (params (Actor :type "Actor Object Reference") (Stimulus :type "AIStimulus Structure")))

(event `self.AIPerception.OnTargetPerceptionInfoUpdated`
  (params (UpdateInfo :type "ActorPerceptionUpdateInfo Structure (by ref)"))
  (bind (_targetid _target _stimulus) (break `ActorPerceptionUpdateInfo` UpdateInfo))
  (`self.HandlePerception` _target _stimulus))

(event `self.NewWeaponEquipped`
  (params (`New Weapon Type` :type "/Game/1_AIAG_Shooter/Enums/ENUM_WeaponType Enum" :default "NewEnumerator0") (`New Weapon Class` :type "/Game/1_AIAG_Shooter/Enums/ENUM_Weapons Enum" :default "NewEnumerator0"))
  (if (not (`|EnumEquality` `New Weapon Type` "NewEnumerator1"))
    (`self.ClearBlackboardValue` "WeaponPadPosition")))

(event `self.PossessedCharacterDied`
  (params (Attacker :type "Actor Object Reference"))
  (`self.ClearBlackboardValue` "SoundPosition")
  (`self.ClearBlackboardValue` "HealthPadPosition")
  (`self.ClearBlackboardValue` "LowHealth")
  (`self.ClearBlackboardValue` "WeaponPadPosition")
  (`self.ClearBlackboardValue` "Target"))

(fn `CalculateDistanceFromAgent`
  (params (Actor :type "Actor Object Reference"))
  (returns (Distance :type "Float (double-precision)"))
  (return (`KismetMathLibrary.Vector_Distance` (`self.K2_GetActorLocation` (`self.GetControlledHero`)) (`self.K2_GetActorLocation` Actor))))

(fn `CheckWeaponPad`
  (params (WeaponPad :type "/Game/1_AIAG_Shooter/Blueprints/BP_SpawnPad_Weapon Object Reference"))
  (locals (Pad :type "/Game/1_AIAG_Shooter/Blueprints/BP_SpawnPad_Weapon Object Reference"))
  (bind (_weapontype _weaponclass) (`/Game/1_AIAG_Shooter/Characters/BP_Hero.Weapon GetEquippedWeaponType` (`self.GetControlledHero`)))
  (bind _output_get (set `local.Pad` WeaponPad))
  (if (`/Game/1_AIAG_Shooter/Blueprints/BP_SpawnPad.IsPickupAvailable?` _output_get)
    (if (`|EnumEquality` _weapontype "NewEnumerator1")
      (`self.SetVectorOnBlackboard` "WeaponPadPosition" (`self.K2_GetActorLocation` _output_get) :!label _label)
      (else
        (if (`|EnumEquality` _weaponclass "NewEnumerator1")
          (bind (_ispickupavailable_ _spawnedweapon) (`/Game/1_AIAG_Shooter/Blueprints/BP_SpawnPad_Weapon.GetSpawnedWeapon` (`local.Pad`)))
          (if (`|EnumEquality` _spawnedweapon "NewEnumerator2")
            (goto _label)
            (else
              _)))
        (`self.ClearBlackboardValue` "WeaponPadPosition" :!label _label_2)))
    (else
      (goto _label_2))))

(fn `ClearBlackboardValue`
  (params (Key :type Name))
  (`BlackboardComponent.ClearValue` (`AIBlueprintHelperLibrary.GetBlackboard` null) Key))

(fn `HandleCharacterDetected`
  (params (Hero :type "/Game/1_AIAG_Shooter/Characters/BP_Hero Object Reference"))
  (locals (Enemy :type "/Game/1_AIAG_Shooter/Characters/BP_Hero Object Reference") (Agent :type "/Game/1_AIAG_Shooter/Characters/BP_Hero Object Reference"))
  (bind _agent (`local.Agent`))
  (bind _enemy (`local.Enemy`))
  (if (`/Game/1_AIAG_Shooter/BT_CheckAffiliationComponent.CheckAffiliationToTarget` (`self.BT_CheckAffiliationComponent`) Hero)
    (set `local.Enemy` Hero)
    (set `local.Agent` (`self.GetControlledHero`))
    (`self.Update Focus Target` _enemy)
    (if (`self.IsEnemyInOptimalRange` _enemy)
      (`/Game/1_AIAG_Shooter/Characters/BP_Hero.Character Set State` _agent "NewEnumerator2")
      (else
        (`/Game/1_AIAG_Shooter/Characters/BP_Hero.Character Set State` _agent "NewEnumerator0")))))

(fn `HandleDamageTaken`
  (params (Attacker :type "Actor Object Reference"))
  (if (`/Game/1_AIAG_Shooter/BT_CheckAffiliationComponent.CheckAffiliationToTarget` (`self.BT_CheckAffiliationComponent`) Attacker)
    (`self.Update Focus Target` Attacker)))

(fn `HandleHearing`
  (params (Stimulus :type "AIStimulus Structure") (Character :type "Actor Object Reference"))
  (if (`/Game/1_AIAG_Shooter/BT_CheckAffiliationComponent.CheckAffiliationToTarget` (`self.BT_CheckAffiliationComponent`) Character)
    (`/Engine/EditorBlueprintResources/StandardMacros.IsValid` (`/Game/1_AIAG_Shooter/Characters/BP_Hero.Character GetFocusTarget` (`self.GetControlledHero`))
      (:`Is Valid`
        (`self.ClearBlackboardValue` "SoundPosition"))
      (:`Is Not Valid`
        (`BlackboardComponent.SetValueAsVector` (`AIBlueprintHelperLibrary.GetBlackboard` null) "SoundPosition" (`.StimulusLocation` (break `AIStimulus` Stimulus)))))))

(fn `HandlePerception`
  (params (SensedActor :type "Actor Object Reference") (AIStimulus :type "AIStimulus Structure (by ref)"))
  (locals (SensedObj :type "Actor Object Reference") (Stimulus :type "AIStimulus Structure") (StimulusClass :type "AISense Class Reference"))
  (bind _stimulusclass (`local.StimulusClass`))
  (set `local.SensedObj` SensedActor)
  (bind _output_get (set `local.Stimulus` AIStimulus))
  (bind _returnvalue (`AIPerceptionSystem.GetSenseClassForStimulus` _output_get))
  (bind _output_get_2 (set `local.StimulusClass` _returnvalue))
  (if (== _output_get_2 "/Script/AIModule.AISense_Damage")
    (`self.UpdateHealthStatus`))
  (if (`.bSuccessfullySensed` (break `AIStimulus` AIStimulus))
    (bind _asbp_hero (cast `/Game/1_AIAG_Shooter/Characters/BP_Hero` (`local.SensedObj`))
      (:`then`
        (if (== _stimulusclass "/Script/AIModule.AISense_Sight")
          (`self.HandleCharacterDetected` _asbp_hero)
          (elif (== _stimulusclass "/Script/AIModule.AISense_Damage")
            (`self.HandleDamageTaken` (`local.SensedObj`)))))
      (:`CastFailed`
        (bind _asbp_spawn_pad_health (cast `/Game/1_AIAG_Shooter/Blueprints/BP_SpawnPad_Health` (`local.SensedObj`))
          (:`then`
            (`self.SetVectorOnBlackboard` "HealthPadPosition" (`self.K2_GetActorLocation` _asbp_spawn_pad_health)))
          (:`CastFailed`
            (bind _asbp_spawn_pad_weapon (cast `/Game/1_AIAG_Shooter/Blueprints/BP_SpawnPad_Weapon` (`local.SensedObj`)))
            (`self.CheckWeaponPad` _asbp_spawn_pad_weapon)))))
    (else
      (bind _returnvalue_2 (`AIPerceptionSystem.GetSenseClassForStimulus` (`local.Stimulus`)))
      (if (== _returnvalue_2 "/Script/AIModule.AISense_Sight")
        (if (== (`local.SensedObj`) (`/Game/1_AIAG_Shooter/Characters/BP_Hero.Character GetFocusTarget` (`self.GetControlledHero`)))
          (`self.ClearFocusTarget`)
          (`self.ClearBlackboardValue` "Target"))
        (`/Game/1_AIAG_Shooter/Characters/BP_Hero.Character Set State` (`self.GetControlledHero`) "NewEnumerator1")
        (elif (== "/Script/AIModule.AISense_Hearing" _returnvalue_2)
          (`self.ClearBlackboardValue` "SoundPosition"))))))

(fn `IsEnemyInOptimalRange`
  (params (Enemy :type "/Game/1_AIAG_Shooter/Characters/BP_Hero Object Reference"))
  (returns (IsInRange :type Boolean))
  (set `self.OptimalRange` (`/Game/1_AIAG_Shooter/Characters/BP_Hero.Weapon GetOptimalRange` (`self.GetControlledHero`)))
  ;[1 1 1] If agent has shotgun, optimal range is fixed on 100
  (if (`|EnumEquality` (`.WeaponClass` (`/Game/1_AIAG_Shooter/Characters/BP_Hero.Weapon GetEquippedWeaponType` (`self.GetControlledHero`))) "NewEnumerator1")
    (set `self.OptimalRange` 100.0))
  (return (<= (`KismetMathLibrary.Vector_Distance` (`self.K2_GetActorLocation` Enemy) (`self.K2_GetActorLocation`)) (`self.OptimalRange`))))

(fn `SetVectorOnBlackboard`
  (params (`Param name` :type Name) (Vector :type "Vector Structure"))
  (`BlackboardComponent.SetValueAsVector` (`AIBlueprintHelperLibrary.GetBlackboard` null) `Param name` Vector))

(fn `Update Focus Target`
  (params (Enemy :type "Actor Object Reference (by ref)"))
  (locals (target :type "Actor Object Reference"))
  (bind _target (`local.target`))
  (bind _focus_target (`/Game/1_AIAG_Shooter/Characters/BP_Hero.Character GetFocusTarget` (`self.GetControlledHero`)))
  (bind _output_get (set `local.target` Enemy))
  (`/Engine/EditorBlueprintResources/StandardMacros.IsValid` _focus_target
    (:`Is Valid`
      (if (< (`self.CalculateDistanceFromAgent` _output_get) (`self.CalculateDistanceFromAgent` _focus_target))
        (`self.SetFocusTarget` _target :!label _label)
        (`BlackboardComponent.SetValueAsObject` (`AIBlueprintHelperLibrary.GetBlackboard` null) "Target" _target)
        (return)))
    (:`Is Not Valid`
      (goto _label))))

(fn `UpdateHealthStatus`
  (bind (_health _maxhealth) (`/Game/1_AIAG_Shooter/Characters/BP_Hero.Character GetHealthStatus` (`self.GetControlledHero`)))
  (`BlackboardComponent.SetValueAsBool` (`AIBlueprintHelperLibrary.GetBlackboard` null) "LowHealth" (<= (/ (* _health 100.0) _maxhealth) 35.0)))

(fn `UserConstructionScript`
  (`parent.UserConstructionScript`))