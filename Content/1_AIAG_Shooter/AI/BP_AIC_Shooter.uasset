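; BP_AIC_Shooter is an AI controller for shooter heroes, caching the possessed BP_Hero on possession.
; It declares empty events for game score updates, teammate and own death, weapon equips, and character launch and landing.
; Focus functions wrap SetFocus and ClearFocus, each calling OnUpdateFocusTarget to broadcast the change.
; Getters expose the controlled hero and team tag.
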(event `self.ReceivePossess`
  (params (PossessedPawn :type "Pawn Object Reference"))
  (bind _asbp_hero (cast `/Game/1_AIAG_Shooter/Characters/BP_Hero` PossessedPawn))
  (set `self.ControlledHero` _asbp_hero))

(event `GameUpdate`
  (params (`My Team Score` :type Integer) (`Enemy Team Highest Score` :type Integer) (TeamWinning :type "GameplayTag Structure")))

(event `TeamMateDied`
  (params (`Team Mate Dead Location` :type "Vector Structure")))

(event `PossessedCharacterDied`
  (params (Attacker :type "Actor Object Reference")))

(event `NewWeaponEquipped`
  (params (`New Weapon Type` :type "/Game/1_AIAG_Shooter/Enums/ENUM_WeaponType Enum" :default "NewEnumerator0") (`New Weapon Class` :type "/Game/1_AIAG_Shooter/Enums/ENUM_Weapons Enum" :default "NewEnumerator0")))

(event `OnCharacterLaunched`)

(event `OnCharacterLanded`)

(fn `ClearFocusTarget`
  (`self.K2_ClearFocus`)
  (`self.OnUpdateFocusTarget` null))

(fn `GetControlledHero`
  (returns (ControlledHero :type "/Game/1_AIAG_Shooter/Characters/BP_Hero Object Reference"))
  (return (`self.ControlledHero`)))

(fn `GetTeamTag`
  (returns (TeamTag :type "GameplayTag Structure"))
  (return (`self.TeamTag`)))

(fn `SetFocusTarget`
  (params (NewFocus :type "Actor Object Reference"))
  (`self.K2_SetFocus` NewFocus)
  (`self.OnUpdateFocusTarget` NewFocus))

(fn `UserConstructionScript`)