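; AI-controlled team shooter character with health, an equippable weapon, movement states and a team-colored body and nameplate.
; On possession it spawns a pistol and follows BP_AIC_Shooter's focus target for firing and aim pitch, adding a distance-scaled offset for short weapons.
; Damage types route to healing or damage, and death unpossesses it and reports killer and controller to the game state.
; Weapon changes and jump-pad launches and landings notify the controller.
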(event `self.ReceivePossessed`
  (params (NewController :type "Controller Object Reference"))
  (bind _asbp_aic_shooter (cast `/Game/1_AIAG_Shooter/AI/BP_AIC_Shooter` NewController))
  (add `/Game/1_AIAG_Shooter/AI/BP_AIC_Shooter.OnUpdateFocusTarget` _asbp_aic_shooter (delegate `OnUpdateFocusTarget_Event`))
  ;[1 1 1] Equip initial weapon when character is possessed
  (bind _returnvalue (`|SpawnActorFromClass` "/Game/3_Weapons/B_Weapon_Pistol.B_Weapon_Pistol_C" (`KismetMathLibrary.MakeTransform` (0.0 0.0 0.0)) "AlwaysSpawn" "SelectDefaultAtRuntime" self null))
  (`self.EquipWeapon` _returnvalue))

(event `OnUpdateFocusTarget_Event`
  (params (`New focus target` :type "Actor Object Reference"))
  (`self.UpdateFocusTarget` `New focus target`))

(event `self.ReceiveBeginPlay`
  (`self.Initialization`))

(event `self.ReceiveTick`
  (params (DeltaSeconds :type "Float (single-precision)"))
  (bind (_returnvalue_x _returnvalue_y _returnvalue_z) (`KismetMathLibrary.BreakVector` (`self.K2_GetActorLocation` (`self.Focus Target`))))
  (if (and (`KismetSystemLibrary.IsValid` (`self.EquippedWeapon`)) (`KismetSystemLibrary.IsValid` (`self.Focus Target`)))
    (set `self.AimPitch` (.pitch (`KismetMathLibrary.FindLookAtRotation` (`self.K2_GetActorLocation` (`self.EquippedWeapon`)) (`KismetMathLibrary.MakeVector` _returnvalue_x _returnvalue_y (select `/Game/1_AIAG_Shooter/Enums/ENUM_WeaponType` (`/Game/3_Weapons/B_Weapon.WeaponType` (`self.EquippedWeapon`)) :`NewEnumerator0` _returnvalue_z :`NewEnumerator1` (select `bool` (> (`self.GetDistanceTo` (`self.Focus Target`)) 500.0) :`false` _returnvalue_z :`true` (+ _returnvalue_z (`KismetMathLibrary.Lerp` -40.0 -150.0 (`KismetMathLibrary.FClamp` (/ (`self.GetDistanceTo` (`self.Focus Target`)) (`/Game/3_Weapons/B_Weapon.WeaponOptimalRange` (`self.EquippedWeapon`))))))))))))
    (else
      (set `self.AimPitch` 0.0)
      (set `self.AimYaw` 0.0))))

(event `self.ReceiveAnyDamage`
  (params (Damage :type "Float (single-precision)") (DamageType :type "DamageType Object Reference") (InstigatedBy :type "Controller Object Reference") (DamageCauser :type "Actor Object Reference"))
  (bind _returnvalue (`GameplayStatics.GetObjectClass` DamageType))
  (if (== (`GameplayStatics.GetObjectClass` DamageType) "/Game/1_AIAG_Shooter/Blueprints/BP_DT_Heal.BP_DT_Heal_C")
    (`self.ReceiveHealth` Damage)
    (elif (or (== _returnvalue "/Game/1_AIAG_Shooter/Blueprints/BP_DT_Damage.BP_DT_Damage_C") (== _returnvalue "/Engine/EngineDamageTypes/DmgTypeBP_Environmental.DmgTypeBP_Environmental_C"))
      (`self.TakeDamage` Damage InstigatedBy DamageCauser))))

(event `self.OnLaunched`
  (params (LaunchVelocity :type "Vector Structure") (bXYOverride :type Boolean) (bZOverride :type Boolean))
  (if (not (`self.Teleporting`))
    ;[1 1 1] jump pads
    (set `self.Launched` true)
    (bind _asbp_aic_shooter (cast `/Game/1_AIAG_Shooter/AI/BP_AIC_Shooter` (`self.GetController`)))
    (`/Game/1_AIAG_Shooter/AI/BP_AIC_Shooter.OnCharacterLaunched` _asbp_aic_shooter)))

(event `self.OnLanded`
  (params (Hit :type "HitResult Structure (by ref)"))
  (if (`self.Teleporting`)
    (set `self.Teleporting` false)
    (elif (`self.Launched`)
      (`self.Character Set State` (`self.CharacterPreviousState`))
      (set `self.Launched` false)
      (bind _asbp_aic_shooter (cast `/Game/1_AIAG_Shooter/AI/BP_AIC_Shooter` (`self.GetController`)))
      (`/Game/1_AIAG_Shooter/AI/BP_AIC_Shooter.OnCharacterLanded` _asbp_aic_shooter))))

(fn `Character GetFocusTarget`
  (returns (`Focus Target` :type "Actor Object Reference"))
  (return (`self.Focus Target`)))

(fn `Character GetHealthStatus`
  (returns (Health :type "Float (double-precision)") (MaxHealth :type "Float (double-precision)") (`Missing Health` :type "Float (double-precision)"))
  (bind _health (`self.Health`))
  (bind _maxhealth (`self.MaxHealth`))
  (return _health _maxhealth (- _maxhealth _health)))

(fn `Character GetTeamTag`
  (returns (TeamTag :type "GameplayTag Structure"))
  (return (`self.TeamTag`)))

(fn `Character Set State`
  (params (`New State` :type "/Game/1_AIAG_Shooter/ENUM_CharacterState Enum" :default "NewEnumerator0"))
  (returns (Success :type Boolean))
  (if (`self.InCrouchTransition`)
    (return false)
    (else
      (if (and (`|EnumInequality` `New State` "NewEnumerator3") (`self.bIsCrouched`))
        (`self.UnCrouch`))
      (set `self.CharacterPreviousState` (`self.CharacterState`))
      (if (and (`|EnumEquality` (`self.CharacterState`) "NewEnumerator3") (`|EnumEquality` `New State` "NewEnumerator3"))
        ;[1 1 1] Update movement speed after crouch transitions freeze movement
        (`self.UpdateMovementSpeed` false)
        (return false)
        (else
          (switch `/Game/1_AIAG_Shooter/ENUM_CharacterState` `New State`
            (:`NewEnumerator0`
              (set `self.CharacterState` "NewEnumerator0")
              (`self.UpdateMovementSpeed` false :!label _label)
              (return true))
            (:`NewEnumerator1`
              (set `self.CharacterState` "NewEnumerator1")
              (goto _label))
            (:`NewEnumerator2`
              (set `self.CharacterState` "NewEnumerator2")
              (goto _label))
            (:`NewEnumerator3`
              (if (and (`self.CanCrouch`) (not (`self.bIsCrouched`)))
                (set `self.CharacterState` "NewEnumerator3")
                (`self.Crouch`)
                (goto _label)))))))))

(fn `Death`
  (params (Killer :type "Actor Object Reference"))
  (locals (AIControllerToKeep :type "/Game/1_AIAG_Shooter/AI/BP_AIC_Shooter Object Reference"))
  (bind _equippedweapon (`self.EquippedWeapon`))
  (bind _aicontrollertokeep (`local.AIControllerToKeep`))
  (set `self.Dead` true)
  (bind _asbp_aic_shooter (cast `/Game/1_AIAG_Shooter/AI/BP_AIC_Shooter` (`self.GetController`)))
  (`/Game/1_AIAG_Shooter/AI/BP_AIC_Shooter.PossessedCharacterDied` _asbp_aic_shooter Killer)
  (`Controller.UnPossess` _asbp_aic_shooter)
  (set `local.AIControllerToKeep` _asbp_aic_shooter)
  (bind _asbp_shooter_game_state (cast `/Game/1_AIAG_Shooter/Blueprints/BP_ShooterGameState` (`GameplayStatics.GetGameState`))
    (:`then`
      ;[1 1 1] Died to another Character?
      (bind _asbp_hero (cast `/Game/1_AIAG_Shooter/Characters/BP_Hero` (`local.Killer`))
        (:`then`
          (`/Game/1_AIAG_Shooter/Blueprints/BP_ShooterGameState.CharacterDied` _asbp_shooter_game_state self null (`/Game/1_AIAG_Shooter/Characters/BP_Hero.TeamTag` _asbp_hero) _aicontrollertokeep))
        (:`CastFailed`
          (`/Game/1_AIAG_Shooter/Blueprints/BP_ShooterGameState.CharacterDied` :`self` _asbp_shooter_game_state :`Hero Killed` self :`Controller Class` _aicontrollertokeep)))
      (`/Engine/EditorBlueprintResources/StandardMacros.IsValid` _equippedweapon
        (:`Is Valid`
          (`self.K2_DestroyActor` _equippedweapon))))
    (:`CastFailed`
      (`KismetSystemLibrary.PrintString` "ERROR! GAME STATE NOT FOUND"))))

(fn `EquipWeapon`
  (params (WeaponToEquip :type "/Game/3_Weapons/B_Weapon Object Reference"))
  (locals (NewLocalVar :type "/Game/3_Weapons/B_Weapon Object Reference"))
  (bind _equippedweapon (`self.EquippedWeapon`))
  (`/Engine/EditorBlueprintResources/StandardMacros.IsValid` WeaponToEquip
    (:`Is Valid`
      (`/Engine/EditorBlueprintResources/StandardMacros.IsValid` (`self.EquippedWeapon`)
        (:`Is Valid`
          (`self.K2_DestroyActor` (`self.EquippedWeapon`)))
        (:`Is Not Valid`
          _))
      (bind _output_get (set `self.EquippedWeapon` (`local.WeaponToEquip`)))
      (bind _returnvalue (`self.K2_AttachToComponent` _output_get (`self.Mesh`) (select `/Game/1_AIAG_Shooter/Enums/ENUM_WeaponType` (`/Game/3_Weapons/B_Weapon.WeaponType` (`self.EquippedWeapon`)) :`NewEnumerator0` "RifleSocket" :`NewEnumerator1` "PistolSocket" :!type "Name") "SnapToTarget" "SnapToTarget" "KeepRelative" true))
      (if _returnvalue
        (bind _asbp_aic_shooter (cast `/Game/1_AIAG_Shooter/AI/BP_AIC_Shooter` (`self.GetController`)))
        (`/Game/1_AIAG_Shooter/AI/BP_AIC_Shooter.NewWeaponEquipped` _asbp_aic_shooter (`/Game/3_Weapons/B_Weapon.WeaponType` _equippedweapon) (`/Game/3_Weapons/B_Weapon.WeaponClass` _equippedweapon))))))

(fn `GetAimData`
  (returns (AimPitch :type "Float (double-precision)") (AimYaw :type "Float (double-precision)"))
  (return (`self.AimPitch`) (`self.AimYaw`)))

(fn `GetEquippedWeapon`
  (returns (EquippedWeapon :type "/Game/3_Weapons/B_Weapon Object Reference"))
  (return (`self.EquippedWeapon`)))

(fn `GetTeleporting`
  (returns (Teleporting :type Boolean))
  (return (`self.Teleporting`)))

(fn `Initialization`
  (set `self.Health` (`self.MaxHealth`))
  (`self.UpdateMovementSpeed` false)
  ;[1 1 1] Initialize nameplate healthbar
  (bind _asw_nameplate (cast `/Game/UI/W_Nameplate` (`WidgetComponent.GetUserWidgetObject` (`self.Widget`))))
  (bind _output_get (set `self.W_Healthbar` _asw_nameplate))
  (`/Game/UI/W_Nameplate.InitializeNameplate` _output_get self (`self.TeamColor`)))

(fn `ReceiveHealth`
  (params (`Heal Ammount` :type "Float (double-precision)"))
  (bind _returnvalue (+ `Heal Ammount` (`self.Health`)))
  (set `self.Health` (select `bool` (> _returnvalue (`self.MaxHealth`)) :`false` _returnvalue :`true` (`self.MaxHealth`)))
  (`/Game/UI/W_Nameplate.SetHealthBarPercent` (`self.W_Healthbar`) (/ (`self.Health`) (`self.MaxHealth`)))
  (return))

(fn `TakeDamage`
  (params (DamageReceived :type "Float (double-precision)") (`Instigated By` :type "Controller Object Reference") (`Damaged By` :type "Actor Object Reference"))
  (locals (DamageAmmount :type "Float (double-precision)") (EnemyDamageDealer :type "Pawn Object Reference"))
  (bind _returnvalue (- (`self.Health`) (`local.DamageAmmount`)))
  (`/Engine/EditorBlueprintResources/StandardMacros.IsValid` `Instigated By`
    (:`Is Valid`
      (set `local.EnemyDamageDealer` (`Controller.K2_GetPawn` `Instigated By`)))
    (:`Is Not Valid`
      _))
  (set `local.DamageAmmount` DamageReceived)
  (set `self.Health` (select `bool` (< _returnvalue 0.0) :`false` _returnvalue))
  (`/Game/UI/W_Nameplate.SetHealthBarPercent` (`self.W_Healthbar`) (/ (`self.Health`) (`self.MaxHealth`)))
  (if (<= (`self.Health`) 0.0)
    (if (not (`self.Dead`))
      (`self.Death` (`local.EnemyDamageDealer`)))
    (else
      (`AISense_Damage.ReportDamageEvent` self (`local.EnemyDamageDealer`) (`local.DamageAmmount`) (`self.K2_GetActorLocation`)))))

(fn `UpdateFocusTarget`
  (params (`New Focus Target` :type "Actor Object Reference"))
  (set `self.Focus Target` `New Focus Target`))

(fn `UpdateMovementSpeed`
  (params (FreezeMovement :type Boolean))
  (bind _charactermovement (`self.CharacterMovement`))
  (bind _output_get (set `self.InCrouchTransition` FreezeMovement))
  (if _output_get
    (set `CharacterMovementComponent.MaxWalkSpeed` 0.0 _charactermovement)
    (set `CharacterMovementComponent.MaxWalkSpeedCrouched` 0.0 _charactermovement)
    (else
      (switch `/Game/1_AIAG_Shooter/ENUM_CharacterState` (`self.CharacterState`)
        (:`NewEnumerator0`
          (set `CharacterMovementComponent.MaxWalkSpeed` (`self.WalkSpeedHipfire`) (`self.CharacterMovement`)))
        (:`NewEnumerator1`
          (set `CharacterMovementComponent.MaxWalkSpeed` (`self.WalkSpeedJogging`) (`self.CharacterMovement`)))
        (:`NewEnumerator2`
          (set `CharacterMovementComponent.MaxWalkSpeed` (`self.WalkSpeedADS`) (`self.CharacterMovement`)))
        (:`NewEnumerator3`
          (set `CharacterMovementComponent.MaxWalkSpeedCrouched` (`self.WalkSpeedCrouched`) (`self.CharacterMovement`)))))))

(fn `UserConstructionScript`
  (bind _mesh (`self.Mesh`))
  (bind _mesh_2 (`self.Mesh`))
  (bind _returnvalue (`PrimitiveComponent.CreateDynamicMaterialInstance` _mesh_2 0 (`PrimitiveComponent.GetMaterial` _mesh_2 0) "None"))
  (set `self.DMI_Body0` _returnvalue)
  (bind _returnvalue_2 (`PrimitiveComponent.CreateDynamicMaterialInstance` _mesh 1 (`PrimitiveComponent.GetMaterial` _mesh 1) "None"))
  (set `self.DMI_Body1` _returnvalue_2)
  (`MaterialInstanceDynamic.SetVectorParameterValue` (`self.DMI_Body0`) "TeamColor" (`self.TeamColor`))
  (`MaterialInstanceDynamic.SetVectorParameterValue` (`self.DMI_Body1`) "TeamColor" (`self.TeamColor`)))

(fn `Weapon CheckRemaining Bullets`
  (returns (NeedsToReload :type Boolean) (RemainingBullets :type Integer))
  (bind _equippedweapon (`self.EquippedWeapon`))
  (bind (_needstoreload _remainingbullets) (`/Game/3_Weapons/B_Weapon.CheckRemainingBullets` _equippedweapon))
  (`/Engine/EditorBlueprintResources/StandardMacros.IsValid` _equippedweapon
    (:`Is Valid`
      (return _needstoreload _remainingbullets))))

(fn `Weapon Fire`
  (bind _equippedweapon (`self.EquippedWeapon`))
  (`/Engine/EditorBlueprintResources/StandardMacros.IsValid` _equippedweapon
    (:`Is Valid`
      (`/Game/3_Weapons/B_Weapon.Fire` _equippedweapon (`self.Focus Target`)))))

(fn `Weapon GetEquippedWeaponType`
  (returns (WeaponType :type "/Game/1_AIAG_Shooter/Enums/ENUM_WeaponType Enum") (WeaponClass :type "/Game/1_AIAG_Shooter/Enums/ENUM_Weapons Enum"))
  (bind _equippedweapon (`self.EquippedWeapon`))
  (return (`/Game/3_Weapons/B_Weapon.WeaponType` _equippedweapon) (`/Game/3_Weapons/B_Weapon.WeaponClass` _equippedweapon)))

(fn `Weapon GetOptimalRange`
  (returns (WeaponOptimalRange :type "Float (double-precision)"))
  (return (`/Game/3_Weapons/B_Weapon.WeaponOptimalRange` (`self.EquippedWeapon`))))

(fn `Weapon Reload`
  (bind _equippedweapon (`self.EquippedWeapon`))
  (`/Engine/EditorBlueprintResources/StandardMacros.IsValid` _equippedweapon
    (:`Is Valid`
      (`/Game/3_Weapons/B_Weapon.Reload` _equippedweapon))))