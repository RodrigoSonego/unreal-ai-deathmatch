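; Nav link launcher that flings BP_Hero agents toward the link's destination when they reach the smart link.
; On arrival it changes the hero's state and launches it, using the raw offset to the destination plus a Z modifier as velocity.
; The construction script applies configurable glow, light and sphere radius settings through a dynamic material and components.
; SwitchActiveState toggles the smart link, dimming the glow and light when disabled.
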(event `self.ReceiveSmartLinkReached`
  (params (Agent :type "Actor Object Reference") (Destination :type "Vector Structure (by ref)"))
  (bind _asbp_hero (cast `/Game/1_AIAG_Shooter/Characters/BP_Hero` Agent))
  (`/Game/1_AIAG_Shooter/Characters/BP_Hero.Character Set State` _asbp_hero "NewEnumerator1")
  (`Character.LaunchCharacter` _asbp_hero (`KismetMathLibrary.MakeVector` (.x (- Destination (`self.K2_GetActorLocation` Agent))) (.y (- Destination (`self.K2_GetActorLocation` Agent))) (+ (.z (- Destination (`self.K2_GetActorLocation` Agent))) (`self.Z Modifier`))) (`self.XYOverride`) (`self.ZOverride`)))

(fn `Switch Active State`
  (params (bEnabled :type Boolean))
  (bind _benabled (`local.bEnabled`))
  (`self.SetSmartLinkEnabled` bEnabled)
  (`MaterialInstanceDynamic.SetScalarParameterValue` (`self.LauncherDynamicMatInst`) "Intensity" (select `bool` _benabled :`false` 1.0 :`true` (`self.Glow Intensity`)))
  (`LightComponent.SetIntensity` (`self.PointLight`) (select `bool` _benabled :`false` 1.0 :`true` (`self.Light Intensity`) :!type "Float (single-precision)")))

(fn `UserConstructionScript`
  (bind _light_color (`self.Light Color`))
  (bind _pointlight (`self.PointLight`))
  (bind _returnvalue (`PrimitiveComponent.CreateDynamicMaterialInstance` (`self.LauncherMesh`) 0 (`PrimitiveComponent.GetMaterial` (`self.LauncherMesh`) 0) "None"))
  (bind _output_get (set `self.LauncherDynamicMatInst` _returnvalue))
  (`MaterialInstanceDynamic.SetScalarParameterValue` _returnvalue "Intensity" (`self.Glow Intensity`))
  (`MaterialInstanceDynamic.SetScalarParameterValue` _output_get "Intensity" (`self.Glow Intensity`))
  (`MaterialInstanceDynamic.SetVectorParameterValueByInfo` _returnvalue (make `MaterialParameterInfo` "Color") _light_color)
  (`LightComponent.SetLightColor` _pointlight _light_color true)
  (`LightComponent.SetIntensity` _pointlight (`self.Light Intensity`))
  (`LocalLightComponent.SetAttenuationRadius` _pointlight (`self.Light Attenuation`))
  (`SphereComponent.SetSphereRadius` (`self.Sphere`) (`self.SphereRadius`) true))