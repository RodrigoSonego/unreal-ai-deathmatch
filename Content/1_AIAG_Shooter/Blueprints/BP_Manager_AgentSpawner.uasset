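; Manager actor that spawns and respawns AI agents for the shooter's three gameplay-tagged teams.
; On BeginPlay it sorts player starts by team; initial population then spawns each team's agents from a data-asset config, cycling through its controller classes and storing controllers per team.
; On agent death it spawns a replacement for the existing controller to possess.
; Spawn points are picked randomly, recursively retrying while occupied, with no retry limit.
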(event `self.ReceiveBeginPlay`
  (bind _outactors (`GameplayStatics.GetAllActorsOfClass` "/Game/1_AIAG_Shooter/Blueprints/BP_ShooterPlayerStart.BP_ShooterPlayerStart_C"))
  (set `self.AllSpawnPoints` _outactors)
  (`self.SetSpawnPointsPerTeam`))

(event `SpawnAgentDied`
  (params (TeamColor :type "LinearColor Structure") (TeamTag :type "GameplayTag Structure") (Controller :type "AIController Object Reference"))
  (bind _freespawnpoint (`self.GetRandomFreeSpawnPoint` (`self.GetSpawnPointsForTeam` TeamTag)))
  (bind _spawned_character (`self.SpawnAgent` _freespawnpoint (`/Game/1_AIAG_Shooter/PDA_TeamConfig.AgentClass` (`self.DA_TeamConfig`)) TeamColor TeamTag))
  (`Controller.Possess` Controller _spawned_character))

(event `SpawnInitialPopulation`
  (bind _da_teamconfig (`self.DA_TeamConfig`))
  (for _array_element (`/Game/1_AIAG_Shooter/PDA_TeamConfig.TeamConfigs` _da_teamconfig)
    (for _ (range 1 (+ (`/Game/1_AIAG_Shooter/PDA_TeamConfig.AgentsPerTeam` _da_teamconfig) 1))
      (bind (_team _teeamcolor _teamcontrollers) (break `/Game/1_AIAG_Shooter/Structs/STRUCT_TeamData` _array_element))
      (if (>= (`self.ControllerIndex`) (`KismetArrayLibrary.Array_Length` _teamcontrollers))
        (set `self.ControllerIndex` 0))
      (bind _freespawnpoint (`self.GetRandomFreeSpawnPoint` (`self.GetSpawnPointsForTeam` _team)))
      (bind _spawned_character (`self.SpawnAgent` _freespawnpoint (`/Game/1_AIAG_Shooter/PDA_TeamConfig.AgentClass` (`self.DA_TeamConfig`)) _teeamcolor _team))
      (bind _spawnedcontroller (`self.SpawnController` (`|GetArrayItem` _teamcontrollers (`self.ControllerIndex`)) _spawned_character _team))
      (`/Engine/EditorBlueprintResources/StandardMacros.IncrementInt` (`self.ControllerIndex`)
        (:`  `
          (`self.StoreAIControllersPerTeam` _spawnedcontroller _team))))
    (`/Engine/EditorBlueprintResources/StandardMacros.IsValid` (`self.GameState`)
      (:`Is Not Valid`
        (cast `/Game/1_AIAG_Shooter/Blueprints/BP_ShooterGameState` (`GameplayStatics.GetGameState`))))))

(fn `GetRandomFreeSpawnPoint`
  (params (SpawnPoints :type "Array of /Game/1_AIAG_Shooter/Blueprints/BP_ShooterPlayerStart Object Reference"))
  (returns (FreeSpawnPoint :type "/Game/1_AIAG_Shooter/Blueprints/BP_ShooterPlayerStart Object Reference"))
  (locals (SpawnPointToCheck :type "/Game/1_AIAG_Shooter/Blueprints/BP_ShooterPlayerStart Object Reference"))
  (bind _output_get (set `local.SpawnPointToCheck` (`KismetArrayLibrary.Array_Random` SpawnPoints)))
  (if (`/Game/1_AIAG_Shooter/Blueprints/BP_ShooterPlayerStart.Occupied` _output_get)
    (bind _freespawnpoint (`self.GetRandomFreeSpawnPoint` (`local.SpawnPoints`)))
    (return _freespawnpoint)
    (else
      (return (`local.SpawnPointToCheck`)))))

(fn `GetSpawnPointsForTeam`
  (params (Selection :type "GameplayTag Structure"))
  (returns (TeamSpawnPoints :type "Array of /Game/1_AIAG_Shooter/Blueprints/BP_ShooterPlayerStart Object Reference"))
  (`|SwitchGameplayTag` Selection
    (:`Shooter.Teams.TeamA`
      (return (`self.TeamASpawnPoints`)))
    (:`Shooter.Teams.TeamB`
      (return (`self.TeamBSpawnPoints`)))
    (:`Shooter.Teams.TeamC`
      (return (`self.TeamCSpawnPoints`)))))

(fn `SetSpawnPointsPerTeam`
  (bind _outactors (`GameplayStatics.GetAllActorsOfClass` "/Game/1_AIAG_Shooter/Blueprints/BP_ShooterPlayerStart.BP_ShooterPlayerStart_C"))
  (for _array_element _outactors
    (`|SwitchGameplayTag` (`/Game/1_AIAG_Shooter/Blueprints/BP_ShooterPlayerStart.Team Tag` _array_element)
      (:`Shooter.Teams.TeamA`
        (`KismetArrayLibrary.Array_AddUnique` (`self.TeamASpawnPoints`) _array_element))
      (:`Shooter.Teams.TeamB`
        (`KismetArrayLibrary.Array_AddUnique` (`self.TeamBSpawnPoints`) _array_element))
      (:`Shooter.Teams.TeamC`
        (`KismetArrayLibrary.Array_AddUnique` (`self.TeamCSpawnPoints`) _array_element)))))

(fn `SpawnAgent`
  (params (SpawnPoint :type "/Game/1_AIAG_Shooter/Blueprints/BP_ShooterPlayerStart Object Reference") (`Character Class` :type "/Game/1_AIAG_Shooter/Characters/BP_Hero Class Reference") (TeamColor :type "LinearColor Structure") (TeamTag :type "GameplayTag Structure"))
  (returns (`Spawned Character` :type "/Game/1_AIAG_Shooter/Characters/BP_Hero Object Reference"))
  (locals (SpawnedAgent :type "/Game/1_AIAG_Shooter/Characters/BP_Hero Object Reference"))
  (bind _returnvalue (`|SpawnActorFromClass` `Character Class` (`self.GetTransform` SpawnPoint) "AlwaysSpawn" "MultiplyWithRoot" null TeamColor TeamTag null))
  (return _returnvalue))

(fn `SpawnController`
  (params (ControllerClass :type "/Game/1_AIAG_Shooter/AI/BP_AIC_Shooter Class Reference") (`Pawn to possess` :type "Pawn Object Reference") (TeamTag :type "GameplayTag Structure"))
  (returns (SpawnedController :type "/Game/1_AIAG_Shooter/AI/BP_AIC_Shooter Object Reference"))
  (bind _returnvalue (`|SpawnActorFromClass` ControllerClass (`self.GetTransform` `Pawn to possess`) "AlwaysSpawn" "MultiplyWithRoot" null TeamTag null))
  (`Controller.Possess` _returnvalue `Pawn to possess`)
  (return _returnvalue))

(fn `StoreAIControllersPerTeam`
  (params (SpawnedAIController :type "/Game/1_AIAG_Shooter/AI/BP_AIC_Shooter Object Reference") (TeamTag :type "GameplayTag Structure"))
  (`KismetArrayLibrary.Array_AddUnique` (`self.AllAIControllers`) SpawnedAIController)
  (`|SwitchGameplayTag` TeamTag
    (:`Shooter.Teams.TeamA`
      (`KismetArrayLibrary.Array_AddUnique` (`self.TeamA_AI_Controllers`) SpawnedAIController))
    (:`Shooter.Teams.TeamB`
      (`KismetArrayLibrary.Array_AddUnique` (`self.TeamB_AI_Controllers`) SpawnedAIController))
    (:`Shooter.Teams.TeamC`
      (`KismetArrayLibrary.Array_AddUnique` (`self.TeamC_AI_Controllers`) SpawnedAIController))))

(fn `UserConstructionScript`)