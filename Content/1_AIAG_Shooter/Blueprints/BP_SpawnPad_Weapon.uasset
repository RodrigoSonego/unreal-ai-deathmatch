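; Weapon spawn pad that offers a randomly chosen weapon, built on a parent pickup class.
; Selection picks a random weapon enum entry, skipping the first, and reads its class and mesh from DT_Weapons by name.
; On pickup, it reloads the character's equipped weapon if the class matches, otherwise spawns and equips the new one, then switches off and starts cooldown.
; GetSpawnedWeapon exposes the current weapon type while the pickup is available.
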(fn `GetSpawnedWeapon`
  (returns (`IsPickupAvailable?` :type Boolean) (SpawnedWeapon :type "/Game/1_AIAG_Shooter/Enums/ENUM_Weapons Enum"))
  (if (`self.IsPickupAvailable?`)
    (return true (`self.PossibleWeapons`))))

(fn `GivePickup`
  (params (`Receiving Character` :type "/Game/1_AIAG_Shooter/Characters/BP_Hero Object Reference"))
  (bind _equippedweapon (`/Game/1_AIAG_Shooter/Characters/BP_Hero.GetEquippedWeapon` `Receiving Character`))
  (bind _receiving_character (`local.Receiving Character`))
  (`parent.GivePickup` `Receiving Character`)
  ;[1 1 1] if same weapon equip, auto reload
  (if (== (`GameplayStatics.GetObjectClass` _equippedweapon) (`self.WeaponToSpawn`))
    (`/Game/3_Weapons/B_Weapon.InsertBulletsIntoMagazine` _equippedweapon)
    (`self.Switch Off` :!label _label)
    (`self.StartCooldown`)
    (else
      (`PrimitiveComponent.SetCollisionEnabled` (`self.Capsule`) "NoCollision")
      (bind _returnvalue (`|SpawnActorFromClass` (`self.WeaponToSpawn`) (`KismetMathLibrary.MakeTransform` (0.0 0.0 0.0)) "AlwaysSpawn" "MultiplyWithRoot" (`local.Receiving Character`) null))
      (`/Engine/EditorBlueprintResources/StandardMacros.IsValid` _receiving_character
        (:`Is Valid`
          (`/Game/1_AIAG_Shooter/Characters/BP_Hero.EquipWeapon` _receiving_character _returnvalue)
          (goto _label))
        (:`Is Not Valid`
          (`self.K2_DestroyActor` _returnvalue)
          (`PrimitiveComponent.SetCollisionEnabled` (`self.Capsule`) "QueryOnly"))))))

(fn `SelectPickupToSpawn`
  (returns (Sucess :type Boolean))
  (bind _output_get (set `self.PossibleWeapons` (cast `/Game/1_AIAG_Shooter/Enums/ENUM_Weapons` (`KismetMathLibrary.Conv_IntToByte` (`KismetMathLibrary.RandomIntegerInRange` 1 (- (enumcount `/Game/1_AIAG_Shooter/Enums/ENUM_Weapons`) 1))))))
  (bind _returnvalue (`|GetDataTableRow` "/Game/1_AIAG_Shooter/Weapons/DT_Weapons.DT_Weapons" (`KismetStringLibrary.Conv_StringToName` (`|GetEnumeratorNameAsString` _output_get)))
    (:`then`
      (bind (_weaponclass _weaponmesh) (break `/Game/1_AIAG_Shooter/Structs/STRUCT_WeaponData` _returnvalue))
      (set `self.WeaponToSpawn` _weaponclass)
      (`StaticMeshComponent.SetStaticMesh` (`self.Pickup Mesh`) _weaponmesh)
      (return true))
    (:`RowNotFound`
      (`KismetSystemLibrary.PrintString` "WARNING: DT ROW NOT FOUND IN WEAPON SPAWNER" true true (struct :`R` 1.0 :`B` 0.005584 :`A` 1.0) 10.0)
      (return false))))

(fn `UserConstructionScript`
  (`parent.UserConstructionScript`))