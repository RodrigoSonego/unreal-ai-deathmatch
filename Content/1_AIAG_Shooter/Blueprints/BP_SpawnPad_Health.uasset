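; BP_SpawnPad_Health is a health pickup spawn pad that overrides or extends a parent pad's pickup logic.
; SelectPickupToSpawn randomly picks a full or partial healthpack, setting both mesh and heal amount.
; GivePickup heals characters below max health through ApplyDamage with a heal damage type, then switches off and starts cooldown.
; GetHealthPackSize reports the heal amount, or zero when the pickup is unavailable.
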(fn `GetHealthPackSize`
  (returns (HealthToGive :type "Float (double-precision)"))
  (if (`self.IsPickupAvailable?`)
    (return (`self.HealthToGive`))
    (else
      (return 0.0))))

(fn `GivePickup`
  (params (`Receiving Character` :type "/Game/1_AIAG_Shooter/Characters/BP_Hero Object Reference"))
  (locals (random :type Boolean :default false))
  (bind (_health _maxhealth) (`/Game/1_AIAG_Shooter/Characters/BP_Hero.Character GetHealthStatus` `Receiving Character`))
  (`/Engine/EditorBlueprintResources/StandardMacros.IsValid` `Receiving Character`
    (:`Is Valid`
      (if (< _health _maxhealth)
        (`GameplayStatics.ApplyDamage` `Receiving Character` (`self.HealthToGive`) (`Pawn.GetController` `Receiving Character`) self "/Game/1_AIAG_Shooter/Blueprints/BP_DT_Heal.BP_DT_Heal_C")
        (`self.Switch Off`)
        (`self.StartCooldown`)))
    (:`Is Not Valid`
      (return))))

(fn `SelectPickupToSpawn`
  (returns (Sucess :type Boolean))
  (locals (random :type Boolean))
  (set `local.random` (`KismetMathLibrary.RandomBool`))
  (`StaticMeshComponent.SetStaticMesh` (`self.Pickup Mesh`) (select `bool` (`local.random`) :`false` "/Game/3_Weapons/Healthpack/Mesh/SM_healthpackPart.SM_healthpackPart" :`true` "/Game/3_Weapons/Healthpack/Mesh/SM_healthpackFull.SM_healthpackFull" :!type "StaticMesh Object Reference"))
  (set `self.HealthToGive` (select `bool` (`local.random`) :`false` 40.0 :`true` 80.0))
  (return true))

(fn `UserConstructionScript`
  (`parent.UserConstructionScript`))